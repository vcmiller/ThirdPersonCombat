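; BP_GiantMan is a giant melee enemy that chases the player and attacks with either hand.
; On BeginPlay it loops AIMoveTo toward the player, setting Attacking and a random AttackType on each success, then waiting before moving again.
; Hand overlaps feed a shared Hit event, which damages the ThirdPersonCharacter only if AttackDamage is set and the hand matches AttackType.
; Hit then clears AttackDamage, which nothing in these graphs sets true.
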(event OnComponentBeginOverlap(LeftHand)
  (params (OverlappedComponent :type Primitive%20Component%20Object%20Reference) (OtherActor :type Actor%20Object%20Reference) (OtherComp :type Primitive%20Component%20Object%20Reference) (OtherBodyIndex :type Integer) (bFromSweep :type Boolean) (SweepResult :type Hit%20Result%20Structure%20%28by%20ref%29))
  (CallFunction|Hit OtherActor))

(event OnComponentBeginOverlap(RightHand)
  (params (OverlappedComponent :type Primitive%20Component%20Object%20Reference) (OtherActor :type Actor%20Object%20Reference) (OtherComp :type Primitive%20Component%20Object%20Reference) (OtherBodyIndex :type Integer) (bFromSweep :type Boolean) (SweepResult :type Hit%20Result%20Structure%20%28by%20ref%29))
  (CallFunction|Hit OtherActor 1))

(event Custom|Hit
  (params (Other :type Actor%20Object%20Reference) (Hand :type Integer))
  (if (and (Variables|Default|GetAttackDamage) (== Hand (Variables|Default|GetAttackType)))
    (bind _asthird_person_character (Utilities|Casting|CastToThirdPersonCharacter Other))
    (Game|Damage|ApplyDamage _asthird_person_character (Variables|Default|GetDamage) 0 0)
    (Variables|Default|SetAttackDamage false)))

(event EventBeginPlay
  (AI|AIMoveTo self "0, 0, 0" (Game|GetPlayerCharacter 0) 2e+02 true :!label _label
    (:OnSuccess
      (Variables|Default|SetAttacking true)
      (Variables|Default|SetAttackType (Math|Random|RandomInteger 2))
      (Utilities|FlowControl|Delay 3.0)
      (goto _label))))

(fn ConstructionScript)